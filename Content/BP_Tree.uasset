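; BP_Tree is a tree the player can cut to collect wood.
; ShowText creates a BP_ActionBubble widget labelled "Cut" and adds it to the viewport, without storing or removing it.
; Action casts the player character to BP_Player and increments its Wood count, leaving the tree itself unchanged.
; Its events and construction script are empty, so both functions rely on external callers.
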(event `self.ReceiveBeginPlay`)

(event `self.ReceiveTick`
  (params (DeltaSeconds :type "Float (single-precision)")))

(fn `Action`
  (bind _asbp_player (cast `/Game/BP_Player` (`GameplayStatics.GetPlayerCharacter` 0)))
  (set `/Game/BP_Player.Wood` (+ (`/Game/BP_Player.Wood` _asbp_player) 1) _asbp_player))

(fn `ShowText`
  (bind _returnvalue (`|CreateWidget` "/Game/BP_ActionBubble.BP_ActionBubble_C" (`GameplayStatics.GetPlayerController` 0)))
  (`TextBlock.SetText` (`/Game/BP_ActionBubble.ActionText_Text` _returnvalue) "Cut")
  (`UserWidget.AddToViewport` _returnvalue 0))

(fn `UserConstructionScript`)